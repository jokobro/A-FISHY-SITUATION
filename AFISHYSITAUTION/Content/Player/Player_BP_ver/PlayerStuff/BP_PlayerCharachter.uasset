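; Player character Blueprint with axis-driven movement and look, plus hardcoded keys that drive the quest system.
; BeginPlay adds the Interactables_UI widget to the viewport as the HUD.
; Every Tick re-finds BP_ServiceManager with GetActorOfClass and calls its quest auto-start.
; X starts the first DT_Quests row, while C, T and Y complete the first three objectives of the "HELPME" row through the manager.
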(event EventBeginPlay
  ;[0.15 0.15 0.15 0.5] Initialize Ui
  (bind _returnvalue (UserInterface|CreateWidget "/Game/UI/Interactables_UI.Interactables_UI_C"))
  (bind _output_get (Variables|Default|SetHud _returnvalue))
  (UserInterface|Viewport|AddtoViewport _output_get 0))

(event Collision|EventActorBeginOverlap
  (params (OtherActor :type Actor%20Object%20Reference)))

(event EventTick
  (params (DeltaSeconds :type Float%20%28single-precision%29))
  ;[0.15 0.15 0.15 0.5] ServiceManager Refrence
  (bind _returnvalue (Actor|GetActorOfClass "/Game/Teshawn/Quest/BP/BP_ServiceManager.BP_ServiceManager_C"))
  (bind _output_get (Variables|Default|SetServiceManager _returnvalue))
  ;[0.15 0.15 0.15 0.5] AutoStart
  (Default|SMAutoStartQuest _output_get))

(event Input|AxisEvents|InputAxisForwards
  (params (AxisValue :type Float%20%28single-precision%29))
  (Pawn|Input|AddMovementInput (Math|Vector|GetForwardVector (Variables|Collision|GetCapsuleComponent)) AxisValue false))

(event Input|AxisEvents|InputAxisRight
  (params (AxisValue :type Float%20%28single-precision%29))
  (Pawn|Input|AddMovementInput (Math|Vector|GetRightVector (Variables|Collision|GetCapsuleComponent)) AxisValue false))

(event Input|AxisEvents|InputAxisTurn
  (params (AxisValue :type Float%20%28single-precision%29))
  (Pawn|Input|AddControllerYawInput AxisValue))

(event Input|AxisEvents|InputAxisLookUp
  (params (AxisValue :type Float%20%28single-precision%29))
  (Pawn|Input|AddControllerPitchInput AxisValue))

(event Input|KeyboardEvents|X
  (params (Key :type Key%20Structure :default "None"))
  (:Pressed
    (bind _outrownames (DataTable|GetDataTableRowNames "/Game/Teshawn/Quest/DataTable/DT_Quests.DT_Quests"))
    (Default|SMSTartQuest (Variables|Default|GetServiceManager) (Utilities|Array|Get(acopy) _outrownames))))

(event Input|KeyboardEvents|C
  (params (Key :type Key%20Structure :default "None"))
  (:Pressed
    ;[0.15 0.15 0.15 0.5] For Completeing a quest
    (bind _returnvalue (Utilities|GetDataTableRow "/Game/Teshawn/Quest/DataTable/DT_Quests.DT_Quests" "HELPME")
      (:then
        (Default|SMCompleteObjective (Variables|Default|GetServiceManager) (.QuestID (Utilities|Struct|BreakS_QuestData _returnvalue)) (.ID (Utilities|Struct|BreakS_Objective (Utilities|Array|Get(acopy) (.Objectives (Utilities|Struct|BreakS_QuestData _returnvalue))))))))))

(event Input|KeyboardEvents|T
  (params (Key :type Key%20Structure :default "None"))
  (:Pressed
    (bind _returnvalue (Utilities|GetDataTableRow "/Game/Teshawn/Quest/DataTable/DT_Quests.DT_Quests" "HELPME")
      (:then
        (Default|SMCompleteObjective (Variables|Default|GetServiceManager) (.QuestID (Utilities|Struct|BreakS_QuestData _returnvalue)) (.ID (Utilities|Struct|BreakS_Objective (Utilities|Array|Get(acopy) (.Objectives (Utilities|Struct|BreakS_QuestData _returnvalue)) 1))))))))

(event Input|KeyboardEvents|Y
  (params (Key :type Key%20Structure :default "None"))
  (:Pressed
    (bind _returnvalue (Utilities|GetDataTableRow "/Game/Teshawn/Quest/DataTable/DT_Quests.DT_Quests" "HELPME")
      (:then
        (Default|SMCompleteObjective (Variables|Default|GetServiceManager) (.QuestID (Utilities|Struct|BreakS_QuestData _returnvalue)) (.ID (Utilities|Struct|BreakS_Objective (Utilities|Array|Get(acopy) (.Objectives (Utilities|Struct|BreakS_QuestData _returnvalue)) 2))))))))

(fn ConstructionScript)