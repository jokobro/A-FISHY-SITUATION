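; BP_Dialogue is an interactable Blueprint that steps through data-table-driven NPC dialogue, one line per TalkingtoNPC call.
; The first call creates a User_Dialogue widget showing the speaker name and line, and later calls update its text.
; Each row supplies the next row name and data table, so conversations chain across tables.
; A row's end flag makes the following call remove and clear the widget.
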(event EventTalkingtoNPC
  (params (playerpref :type BP%20Player%20Object%20Reference))
  (if (Variables|Default|GetEnd_Dialoge)
    (Widget|RemovefromParent (Variables|Default|GetDialogueWidgit))
    (Variables|Default|SetEnd_Dialoge false)
    (Variables|Default|SetDialogueWidgit 0)
    (else
      (Utilities|IsValid (Variables|Default|GetDialogueWidgit)
        (:Is%20Valid
          (bind _returnvalue (Utilities|GetDataTableRow (Variables|Default|GetData%20Table) (Variables|Default|GetRow%20Name))
            (:then
              (Default|UpdateDialogue (Variables|Default|GetDialogueWidgit) (.Dialogue (Utilities|Struct|BreakDIalogue_Structure _returnvalue)))
              (Variables|Default|SetRow%20Name (.Row (Utilities|Struct|BreakDIalogue_Structure _returnvalue)))
              (Variables|Default|SetData%20Table (.Datatable (Utilities|Struct|BreakDIalogue_Structure _returnvalue)))
              (Variables|Default|SetEnd_Dialoge (.End_Dialoge (Utilities|Struct|BreakDIalogue_Structure _returnvalue))))))
        (:Is%20Not%20Valid
          (bind _returnvalue_2 (Utilities|GetDataTableRow (Variables|Default|GetData%20Table) (Variables|Default|GetRow%20Name))
            (:then
              (bind _returnvalue_3 (UserInterface|CreateWidget "/Game/Player/Player_BP_ver/User_Dialogue.User_Dialogue_C" 0 (Utilities|Text|ToText(Name) (Variables|Default|GetName)) (.Dialogue (Utilities|Struct|BreakDIalogue_Structure _returnvalue_2))))
              (Variables|Default|SetDialogueWidgit _returnvalue_3)
              (UserInterface|Viewport|AddtoViewport _returnvalue_3 0)
              (Variables|Default|SetRow%20Name (.Row (Utilities|Struct|BreakDIalogue_Structure _returnvalue_2)))
              (Variables|Default|SetData%20Table (.Datatable (Utilities|Struct|BreakDIalogue_Structure _returnvalue_2)))
              (Variables|Default|SetEnd_Dialoge (.End_Dialoge (Utilities|Struct|BreakDIalogue_Structure _returnvalue_2))))))))))