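; NPC actor Blueprint with a Talk event meant for stepping through dialogue lines, though the event is currently empty.
; Disconnected logic increments TalkIndex, prints the current Dialogue entry, lazily creates a UI widget and clears its TalkText.
; The same unwired branch removes the widget once the index passes the last line, so none of this dialogue flow runs.
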(event EventTalk)

(fn ConstructionScript)