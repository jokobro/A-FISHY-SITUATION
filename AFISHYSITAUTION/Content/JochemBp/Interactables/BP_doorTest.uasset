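; Test interactable door that swings open or closed around its yaw axis each time it is interacted with.
; After a short delay, the Interacted event checks the HasBeenOpenend flag to choose OpenDoor or CloseDoor, with a debug print on closing.
; Each event plays its own timeline to lerp the static mesh's relative rotation through a quarter turn, setting the flag on every update.
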(event Custom|OpenDoor
  ;[0.15 0.15 0.15 0.5] Open and Closing the door
  (bind _doorfloat (Timeline|Open%20Door%20TImeline PlayFromStart)
    (:Update
      (Transformation|SetRelativeRotation (Variables|Default|GetStaticMesh) (Math|Rotator|MakeRotator 0.0 0.0 (Math|Float|Lerp 0.0 9e+01 _doorfloat)) false false)
      (Variables|Default|SetHasBeenOpenend true))))

(event Custom|CloseDoor
  ;[0.15 0.15 0.15 0.5] Open and Closing the door
  (bind _doorfloat (Timeline|Timeline PlayFromStart)
    (:Update
      (Transformation|SetRelativeRotation (Variables|Default|GetStaticMesh) (Math|Rotator|MakeRotator 0.0 0.0 (Math|Float|Lerp 9e+01 0.0 _doorfloat)) false false)
      (Variables|Default|SetHasBeenOpenend false))))

(event EventBeginPlay
  (|CallParentFunction) ; This node is disabled and will not be called.\nDrag off pins to build functionality.
)

(event EventInteracted
  ;[0.15 0.15 0.15 0.5] Handle Opening or Closing of door
  (Utilities|FlowControl|Delay 1.0)
  (if (Variables|Default|GetHasBeenOpenend)
    (CallFunction|CloseDoor)
    (Development|PrintString "ik sluit deur")
    (else
      (CallFunction|OpenDoor))))

(fn ConstructionScript
  (|CallParentFunction))