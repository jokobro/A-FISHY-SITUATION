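; BP_NPC is an interactable NPC that shows dialogue from a DataTable in a User_Dialogue1 widget when interacted with.
; Each row supplies the text plus the next row and table, so a later conversation continues from there.
; While dialogue is open, interacting calls CheckWigetstate, which skips the typewriter effect or, if already skipped, removes the widget.
; The IsValid branch only looks up a row, leaving its state updates unconnected.
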(event EventBeginPlay
  (|CallParentFunction) ; This node is disabled and will not be called.\nDrag off pins to build functionality.
)

(event Collision|EventActorBeginOverlap
  (params (OtherActor :type Actor%20Object%20Reference)))

(event EventTick
  (params (DeltaSeconds :type Float%20%28single-precision%29)))

(event EventInteracted
  (if (Variables|Default|GetEnd_Dialoge)
    (CallFunction|CheckWigetstate)
    (else
      (Utilities|IsValid 0
        (:Is%20Valid
          (bind _returnvalue (Utilities|GetDataTableRow (Variables|Default|GetData%20Table) (Variables|Default|GetRow%20Name))))
        (:Is%20Not%20Valid
          (bind _returnvalue_2 (Utilities|GetDataTableRow (Variables|Default|GetData%20Table) (Variables|Default|GetRow%20Name))
            (:then
              (bind _returnvalue_3 (UserInterface|CreateWidget "/Game/Player/Player_BP_ver/Dialogue/UserDialogue/User_Dialogue1.User_Dialogue1_C" 0 (Utilities|Text|ToText(Name) (Variables|Default|GetName)) (.Dialogue (Utilities|Struct|BreakDIalogue_Structure _returnvalue_2))))
              (bind _output_get (Variables|Default|SetDialogueWidgit _returnvalue_3))
              (UserInterface|Viewport|AddtoViewport _output_get 0)
              (Variables|Default|SetRow%20Name (.Row (Utilities|Struct|BreakDIalogue_Structure _returnvalue_2)))
              (Variables|Default|SetData%20Table (.Datatable (Utilities|Struct|BreakDIalogue_Structure _returnvalue_2)))
              (Variables|Default|SetEnd_Dialoge true))))))))

(fn ConstructionScript
  (|CallParentFunction))

(fn CheckWigetstate
  (if (Variables|/Game/Player/Player_BP_ver/Dialogue/UserDialogue/User_Dialogue1.User_Dialogue1_C|GetSkipTypewriter (Variables|Default|GetDialogueWidgit))
    (Widget|RemovefromParent (Variables|Default|GetDialogueWidgit))
    (Variables|Default|SetDialogueWidgit 0)
    (Variables|Default|SetEnd_Dialoge false)
    (else
      (Default|SkipText (Variables|Default|GetDialogueWidgit))
      (Variables|Default|SetEnd_Dialoge true)))
  (return))