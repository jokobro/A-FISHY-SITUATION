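; BP_RepairObject is an interactable object that can be broken and then repaired after a delay.
; BreakObject flags it as broken and activates the PSmoke effect.
; Interacting while it is broken marks it as repairing and starts a RepairTime timer, without checking whether a repair is already running.
; When the timer fires, FinishRepair clears both flags, deactivates the smoke, prints a debug message and invalidates the timer.
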(event Custom|FinishRepair
  (Variables|Default|SetIsBroken false)
  (Variables|Default|SetIsRepairing false)
  (Development|PrintString "REPAIRED")
  (Components|Activation|Deactivate (Variables|Default|GetP_Smoke))
  (Utilities|Time|ClearandInvalidateTimerbyHandle (stale EventInteracted _output_get)))

(event EventBeginPlay
  (|CallParentFunction))

(event Collision|EventActorBeginOverlap
  (params (OtherActor :type Actor%20Object%20Reference)))

(event EventTick
  (params (DeltaSeconds :type Float%20%28single-precision%29)))

(event EventInteracted
  (if (Variables|Default|GetIsBroken)
    (Variables|Default|SetIsRepairing true)
    (bind _returnvalue (Utilities|Time|SetTimerbyEvent (delegate Custom|FinishRepair) (Variables|Default|GetRepairTime)))
    (bind _output_get (Variables|Default|SetRepairTimerHandle _returnvalue))))

(fn ConstructionScript
  (|CallParentFunction))

(fn BreakObject
  (Variables|Default|SetIsBroken true)
  (Components|Activation|Activate (Variables|Default|GetP_Smoke) false))