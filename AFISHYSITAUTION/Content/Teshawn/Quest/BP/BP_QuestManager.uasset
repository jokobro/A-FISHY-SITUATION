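; Quest manager that tracks active and completed quests with per-quest progress, and shows widgets for quest start, objective completion and quest completion.
; QM-prefixed events start quests from DT_Quests by ID or AutoStart flag, complete objectives and store the active widget.
; Completing an objective rewrites the nested quest structs, then checks every objective to finish the quest.
; Start checks cover completed non-repeatable quests, but the already-active check is unwired.
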(event EventQMAutoSartQuest
  (bind _outrownames (DataTable|GetDataTableRowNames "/Game/Teshawn/Quest/DataTable/DT_Quests.DT_Quests"))
  (for _array_element _outrownames
    (bind _returnvalue (Utilities|GetDataTableRow "/Game/Teshawn/Quest/DataTable/DT_Quests.DT_Quests" _array_element)
      (:then
        (if (.AutoStart (Utilities|Struct|BreakS_QuestData _returnvalue))
          (CallFunction|StartQuest (.QuestID (Utilities|Struct|BreakS_QuestData _returnvalue))))))))

(event EventQMUpdateActiveWidget
  (params (Widget :type Widget%20Object%20Reference))
  (Variables|Default|SetActiveWidget Widget))

(event EventQMStartQuest
  (params (QuestID :type Name :default "None"))
  (CallFunction|StartQuest QuestID))

(event EventQMCompleteObjectives
  (params (QuesrID :type Name :default "None") (ObjectiveID :type Name :default "None"))
  (bind _output (CallFunction|CompleteObjective QuesrID ObjectiveID))
  (if _output
    (CallFunction|CompleteQuest QuesrID)))

(fn ConstructionScript)

(fn StartQuest
  (params (QuestID :type Name))
  (CallFunction|CheckifQuestHasBeenStarted QuestID)
  (if true
    (bind _returnvalue (Utilities|GetDataTableRow "/Game/Teshawn/Quest/DataTable/DT_Quests.DT_Quests" QuestID)
      (:then
        (Utilities|Array|Add (Variables|Default|GetActiveQuests) _returnvalue)
        (Variables|Default|SetQuestProgress (LocalVariables|GetTempProgress))
        (Utilities|Map|Add (LocalVariables|GetTempProgress) QuestID 0)
        (Variables|Default|SetQuestProgress (LocalVariables|GetTempProgress))
        (bind _returnvalue_2 (UserInterface|CreateWidget "/Game/Teshawn/Quest/UI/WB_QuestStarted.WB_QuestStarted_C" 0 _returnvalue))
        (UserInterface|Viewport|AddtoViewport _returnvalue_2 0)))))

(fn CompleteObjective
  (params (QuestID :type Name) (ObjectiveID :type Name))
  (bind _complete_ (CallFunction|ObjectiveCompletion QuestID ObjectiveID))
  (LocalVariables|SettempProgress (Variables|Default|GetQuestProgress))
  (if true
    (bind _result (Math|Integer|IncrementInt (.Value (Utilities|Map|Find (LocalVariables|GettempProgress) QuestID)))
      (:%20%20
        (Utilities|Map|Add (LocalVariables|GettempProgress) QuestID _result)
        (Variables|Default|SetQuestProgress (LocalVariables|GettempProgress))
        (bind _returnvalue (Utilities|GetDataTableRow "/Game/Teshawn/Quest/DataTable/DT_Quests.DT_Quests" QuestID)
          (:then
            (for _array_element (.Objectives (Utilities|Struct|BreakS_QuestData _returnvalue))
              (if (== (.ID (Utilities|Struct|BreakS_Objective _array_element)) ObjectiveID)
                (bind _returnvalue_2 (UserInterface|CreateWidget "/Game/Teshawn/Quest/UI/WB_CompletedObjectibe.WB_CompletedObjectibe_C" 0 _array_element))
                (UserInterface|Viewport|AddtoViewport _returnvalue_2 0)))
            (return _complete_)))))
    (else
      (return false))))

(fn ObjectiveCompletion
  (params (QuestID :type Name) (ObjectiveID :type Name))
  (for (_array_element _array_index) (Variables|Default|GetActiveQuests)
    (LocalVariables|SetTempObjectives (.Objectives (Utilities|Struct|BreakS_QuestData _array_element)))
    (if (== (.QuestID (Utilities|Struct|BreakS_QuestData _array_element)) QuestID)
      (for (_array_element_2 _array_index_2) (.Objectives (Utilities|Struct|BreakS_QuestData _array_element))
        (if (== (.ID (Utilities|Struct|BreakS_Objective _array_element_2)) ObjectiveID)
          (Utilities|Array|SetArrayElem (LocalVariables|GetTempObjectives) _array_index_2 (Utilities|Struct|MakeS_Objective (.ID (Utilities|Struct|BreakS_Objective _array_element_2)) (.Disription (Utilities|Struct|BreakS_Objective _array_element_2)) true (.Type (Utilities|Struct|BreakS_Objective _array_element_2)) (.TargetData (Utilities|Struct|BreakS_Objective _array_element_2)) (.Optional (Utilities|Struct|BreakS_Objective _array_element_2)) (.canCompleteInAnyOrder (Utilities|Struct|BreakS_Objective _array_element_2))))
          (Utilities|Array|SetArrayElem (Variables|Default|GetActiveQuests) _array_index (Utilities|Struct|MakeS_QuestData (.QuestID (Utilities|Struct|BreakS_QuestData _array_element)) (.Tilte (Utilities|Struct|BreakS_QuestData _array_element)) (.Discription (Utilities|Struct|BreakS_QuestData _array_element)) (LocalVariables|GetTempObjectives) (.IsRepeatable (Utilities|Struct|BreakS_QuestData _array_element)) (.AutoStart (Utilities|Struct|BreakS_QuestData _array_element)) (.Rewards (Utilities|Struct|BreakS_QuestData _array_element))))
          (bind _completed (CallFunction|CheckQuestCompleted (.QuestID (Utilities|Struct|BreakS_QuestData _array_element))))
          (return _completed)))
      (else
        (return false)))))

(fn CheckQuestCompleted
  (params (QuestID :type Name))
  (for _array_element (Variables|Default|GetActiveQuests)
    (if (== (.QuestID (Utilities|Struct|BreakS_QuestData _array_element)) QuestID)
      (for _array_element_2 (.Objectives (Utilities|Struct|BreakS_QuestData _array_element))
        (if (not (.IsComplete (Utilities|Struct|BreakS_Objective _array_element_2)))
          (return false)))
      (return true)
      (else
        (return false)))))

(fn CompleteQuest
  (params (QuestID :type Name))
  (for _array_element (Variables|Default|GetActiveQuests)
    (if (== (.QuestID (Utilities|Struct|BreakS_QuestData _array_element)) QuestID)
      (bind _returnvalue (UserInterface|CreateWidget "/Game/Teshawn/Quest/UI/WB_CompletedQuest.WB_CompletedQuest_C" 0 _array_element))
      (UserInterface|Viewport|AddtoViewport _returnvalue 0)
      (Utilities|Array|Add (Variables|Default|GetCompletedQuests) _array_element)
      (Utilities|Array|RemoveItem (Variables|Default|GetActiveQuests) _array_element)
      (Utilities|Map|Remove (Variables|Default|GetQuestProgress) QuestID)
      (return))))

(fn CheckifQuestHasBeenStarted
  (params (QuestID :type Name))
  (for _array_element (Variables|Default|GetCompletedQuests)
    (if (and (== (.QuestID (Utilities|Struct|BreakS_QuestData _array_element)) QuestID) (not (.IsRepeatable (Utilities|Struct|BreakS_QuestData _array_element))))
      (return false)))
  (for _array_element_2 (Variables|Default|GetActiveQuests)
    _))

(fn QMGetActiveQuests
  (return (Variables|Default|GetActiveQuests)))

(fn QMGetActiveWidget
  (return (Variables|Default|GetActiveWidget)))

(fn QMGetCompletedQuests
  (return (Variables|Default|GetCompletedQuests)))