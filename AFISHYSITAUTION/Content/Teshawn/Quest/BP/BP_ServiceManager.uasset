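; BP_ServiceManager is a service facade for the quest system, forwarding quest requests to a QuestManager reference.
; Its events relay starting a quest, completing an objective, auto-starting a quest and setting the active widget as QuestManager messages.
; Its getter functions return the QuestManager's active quests, completed quests and active widget.
; It holds no logic of its own, and the file does not show where QuestManager is assigned.
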(event EventSMAutoStartQuest
  (Class|INTQuestManager|QMAutoSartQuest(Message) (Variables|Default|GetQuestManager)))

(event EventSMSetActiveWidget
  (params (Widget :type Widget%20Object%20Reference))
  (Default|QMUpdateActiveWidget (Variables|Default|GetQuestManager) Widget))

(event EventSMSTartQuest
  (params (QuestID :type Name :default "None"))
  (Class|INTQuestManager|QMStartQuest(Message) (Variables|Default|GetQuestManager) QuestID))

(event EventSMCompleteObjective
  (params (QuestID :type Name :default "None") (ObjectiveID :type Name :default "None"))
  (Class|INTQuestManager|QMCompleteObjectives(Message) (Variables|Default|GetQuestManager) QuestID ObjectiveID))

(fn ConstructionScript)

(fn SMGetActiveQuests
  (bind _activequest (Default|QMGetActiveQuests (Variables|Default|GetQuestManager)))
  (return _activequest))

(fn SMGetActiveWidget
  (bind _widget (Default|QMGetActiveWidget (Variables|Default|GetQuestManager)))
  (return _widget))

(fn SMGetCompletedQuests
  (bind _completedquests (Default|QMGetCompletedQuests (Variables|Default|GetQuestManager)))
  (return _completedquests))